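; BP_Heavy_Infantry is a melee enemy with sight sensing, an attack and health.
; When PawnSensing sees a pawn, it casts that pawn's controller, not its own, to AIC_HeavyInfantry and notifies it of the sighting.
; PerformAttack applies BaseDamage to Target without any range check.
; TakeDamage subtracts damage from Health and destroys the actor at zero or below.
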(event `self.PawnSensing.OnSeePawn`
  (params (Pawn :type "Pawn Object Reference"))
  (bind _asaic_heavy_infantry (cast `/Game/Enemies/MeleeEnemy/HeavyInfantry/AIC_HeavyInfantry` (`self.GetController` Pawn)))
  (`/Game/Enemies/MeleeEnemy/HeavyInfantry/AIC_HeavyInfantry.NotifySeePawn` _asaic_heavy_infantry Pawn))

(event `PerformAttack`
  (`GameplayStatics.ApplyDamage` (`self.Target`) (`self.BaseDamage`)))

(fn `TakeDamage`
  (locals (Damage :type "Float (double-precision)" :default 10.0))
  (bind _output_get (set `self.Health` (- (`self.Health`) (`local.Damage`))))
  (if (<= _output_get 0.0)
    (`self.K2_DestroyActor`)))

(fn `UserConstructionScript`)